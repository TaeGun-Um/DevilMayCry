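; HellCaina enemy Blueprint that supplies montage-based animation events and tracks the enemy's state machine.
; Events play walk, strafe, damaged and death montages at a shared speed, while RandomAttack picks a random montage from the attack array.
; Tick polls HellCainaFsmComp, caches state changes and prints the new state name as debug output.
; Nothing in this graph calls the animation events.
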(event `self.ReceiveTick`
  (params (DeltaSeconds :type "Float (single-precision)"))
  (`self.NewFunction`))

(event `self.RandomAttack`
  (set `self.RandomSeed` (`KismetMathLibrary.RandomInteger` (`KismetArrayLibrary.Array_Length` (`self.AttackArray`))))
  (`self.PlayAnimMontage` (`|GetArrayItem` (`self.AttackArray`) (`self.RandomSeed`)) (`self.AnimSpeed`)))

(event `self.WalkAnimation`
  (`self.PlayAnimMontage` "/Game/Enemy/HellCaina/Anim/Move/BM_Walk.BM_Walk" (`self.AnimSpeed`)))

(event `self.WalkLeftAnimation`
  (`self.PlayAnimMontage` "/Game/Enemy/HellCaina/Anim/Move/BM_Walk_Left.BM_Walk_Left" (`self.AnimSpeed`)))

(event `self.WalkRightAnimation`
  (`self.PlayAnimMontage` "/Game/Enemy/HellCaina/Anim/Move/BM_Walk_Right.BM_Walk_Right" (`self.AnimSpeed`)))

(event `self.DamagedAnimation`
  (`self.PlayAnimMontage` "/Game/Enemy/HellCaina/Anim/Damaged/BM_Damaged.BM_Damaged" (`self.AnimSpeed`)))

(event `self.DeadAnimation`
  (`self.PlayAnimMontage` "/Game/Enemy/HellCaina/Anim/Damaged/BM_DeathFront.BM_DeathFront" (`self.AnimSpeed`)))

(fn `NewFunction`
  (bind _returnvalue (`FsmComponent.GetCurrentState` (`self.HellCainaFsmComp`)))
  (if (!= (`self.CurFsm`) _returnvalue)
    (set `self.CurFsm` _returnvalue)
    (`KismetSystemLibrary.PrintString` (`|GetEnumeratorNameAsString` (cast `EHellCainaFsm` (`KismetMathLibrary.Conv_IntToByte` (`FsmComponent.GetCurrentState` (`self.HellCainaFsmComp`))))))))

(fn `UserConstructionScript`)