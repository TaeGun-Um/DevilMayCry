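; BP_Angelo is the Blueprint for the Angelo enemy character, serving as its animation layer.
; Named events for walking, attacks, warp, parry, damage, stun and death each play a montage at the AnimSpeed rate; none are triggered within this graph.
; FsmCheck is inactive: its disconnected logic would print FsmComp state changes, cast to the EEmpusaFsm enum.
; BeginPlay, Tick and the construction script are empty.
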(event `self.ReceiveBeginPlay`)

(event `self.ReceiveTick`
  (params (DeltaSeconds :type "Float (single-precision)")))

(event `self.DamagedAnimation`
  (`self.PlayAnimMontage` "/Game/Enemy/Angelo/Anim/Damaged/BM_Guard_F.BM_Guard_F" (`self.AnimSpeed`)))

(event `self.DengekiAnimation`
  (`self.PlayAnimMontage` "/Game/Enemy/Angelo/Anim/Attack/BM_Attack_Dengeki.BM_Attack_Dengeki" (`self.AnimSpeed`)))

(event `self.WalkAnimation`
  (`self.PlayAnimMontage` "/Game/Enemy/Angelo/Anim/Move/BM_Walk.BM_Walk" (`self.AnimSpeed`)))

(event `self.RakuraiAnimation`
  (`self.PlayAnimMontage` "/Game/Enemy/Angelo/Anim/Attack/BM_Attack_Rakurai.BM_Attack_Rakurai" (`self.AnimSpeed`)))

(event `self.ParryAnimation`
  (`self.PlayAnimMontage` "/Game/Enemy/Angelo/Anim/Attack/BM_Parry.BM_Parry" (`self.AnimSpeed`)))

(event `self.AttackAnimation`
  (`self.PlayAnimMontage` "/Game/Enemy/Angelo/Anim/Attack/BM_AttackCombo.BM_AttackCombo" (`self.AnimSpeed`) "Attack1"))

(event `self.WarpAnimation`
  (`self.PlayAnimMontage` "/Game/Enemy/Angelo/Anim/Move/BM_Warp.BM_Warp" (`self.AnimSpeed`)))

(event `self.StunAnimation`
  (`self.PlayAnimMontage` "/Game/Enemy/Angelo/Anim/Damaged/BM_Stun.BM_Stun" (`self.AnimSpeed`)))

(event `self.DeadAnimation`
  (`self.PlayAnimMontage` "/Game/Enemy/Angelo/Anim/Damaged/BM_DeathFront.BM_DeathFront" (`self.AnimSpeed`)))

(fn `FsmCheck`)

(fn `UserConstructionScript`)