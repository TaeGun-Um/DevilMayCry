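; BP_Last is an enemy AI controller that runs the BT_Empusa behavior tree on possess.
; Perception updates set a found-target flag and target actor on the Blackboard when an actor tagged Player is sensed.
; Any other update, including another actor being sensed, clears both keys.
; Debug strings print on each perception update and every tick.
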(event `self.ReceiveBeginPlay`)

(event `self.ReceiveTick`
  (params (DeltaSeconds :type "Float (single-precision)"))
  (`KismetSystemLibrary.PrintString` "Hello"))

(event `self.AIPerception.OnTargetPerceptionUpdated`
  (params (Actor :type "Actor Object Reference") (Stimulus :type "AIStimulus Structure"))
  (if (and (`self.ActorHasTag` Actor "Player") (`.bSuccessfullySensed` (break `AIStimulus` Stimulus)))
    (`BlackboardComponent.SetValueAsBool` (`self.Blackboard`) (`self.bFindTarget`) true)
    (`BlackboardComponent.SetValueAsObject` (`self.Blackboard`) (`self.TargetActor`) Actor)
    (`KismetSystemLibrary.PrintString` "FindSuccess")
    (else
      (`BlackboardComponent.SetValueAsBool` (`self.Blackboard`) (`self.bFindTarget`) false)
      (`BlackboardComponent.SetValueAsObject` (`self.Blackboard`) (`self.TargetActor`) null)
      (`KismetSystemLibrary.PrintString` "FindFail"))))

(event `self.ReceivePossess`
  (params (PossessedPawn :type "Pawn Object Reference"))
  (`self.RunBehaviorTree` "/Game/Enemy/Empusa/BT_Empusa.BT_Empusa"))

(fn `UserConstructionScript`)