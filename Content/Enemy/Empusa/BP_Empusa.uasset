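; Empusa enemy Blueprint that plays animation montages for attack, damaged, walk, run, death and snatch events at a shared AnimSpeed.
; RandomAttack picks a random montage from AttackArray and sets CollisionNum to the matching right, left or all collision from EEmpusaCollision.
; No event here is called within the graph, and BeginPlay, Tick and overlap are empty.
; An FsmCheck debug print of EmpusaFsmComp's state is left disconnected.
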(event `self.ReceiveBeginPlay`)

(event `self.ReceiveActorBeginOverlap`
  (params (OtherActor :type "Actor Object Reference")))

(event `self.ReceiveTick`
  (params (DeltaSeconds :type "Float (single-precision)")))

(event `self.RandomAttack`
  (bind _output_get (set `self.RandomSeed` (`KismetMathLibrary.RandomInteger` (`KismetArrayLibrary.Array_Length` (`self.AttackArray`)))))
  (`self.PlayAnimMontage` (`|GetArrayItem` (`self.AttackArray`) (`self.RandomSeed`)) (`self.AnimSpeed`))
  (switch `int` _output_get
    (:`0`
      (set `self.CollisionNum` (`KismetMathLibrary.Conv_ByteToInt` (enumliteral `EEmpusaCollision` "RIGHT"))))
    (:`1`
      (set `self.CollisionNum` (`KismetMathLibrary.Conv_ByteToInt` (enumliteral `EEmpusaCollision` "LEFT"))))
    (:`2`
      (set `self.CollisionNum` (`KismetMathLibrary.Conv_ByteToInt` (enumliteral `EEmpusaCollision` "RIGHT"))))
    (:`3`
      (set `self.CollisionNum` (`KismetMathLibrary.Conv_ByteToInt` (enumliteral `EEmpusaCollision` "ALL"))))
    (:`4`
      (set `self.CollisionNum` (`KismetMathLibrary.Conv_ByteToInt` (enumliteral `EEmpusaCollision` "ALL"))))))

(event `self.DamagedAnimation`
  (`self.PlayAnimMontage` "/Game/Enemy/Empusa/Anim/Damaged/BS_DamagedBack.BS_DamagedBack" (`self.AnimSpeed`)))

(event `self.WalkAnimation`
  (`self.PlayAnimMontage` "/Game/Enemy/Empusa/Anim/Move/BM_Walk.BM_Walk" (`self.AnimSpeed`)))

(event `self.RunAnimation`
  (`self.PlayAnimMontage` "/Game/Enemy/Empusa/Anim/Move/BM_Run.BM_Run" (`self.AnimSpeed`)))

(event `self.DeadAnimation`
  (`self.PlayAnimMontage` "/Game/Enemy/Empusa/Anim/Damaged/BM_DeathFront.BM_DeathFront" (`self.AnimSpeed`)))

(event `self.SnatchAnimation`
  (`self.PlayAnimMontage` "/Game/Enemy/Empusa/Anim/Damaged/BM_EmpusaSnatch.BM_EmpusaSnatch" (`self.AnimSpeed`)))

(fn `FsmCheck`)

(fn `UserConstructionScript`)