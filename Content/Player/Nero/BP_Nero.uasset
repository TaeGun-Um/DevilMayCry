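; BP_Nero is the Blueprint for the player character Nero, handling montage-driven combat actions and enemy lock-on selection.
; Custom events gate Red Queen and jump combos, directional evades, and Overture arm attacks on player state, then play montages and change state.
; Shoot and damage reaction events play montages, with some air/ground variants.
; EnemyCheck selects the nearest living EnemyBase by sphere overlap, then calls an obstacle line trace whose result it ignores.
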(event `self.ReceiveActorBeginOverlap`
  (params (OtherActor :type "Actor Object Reference")))

(event `self.ReceiveTick`
  (params (DeltaSeconds :type "Float (single-precision)")))

(event `self.RedQueenCombo`
  (bind _returnvalue (`self.BlueprintGetCurState`))
  (if (not (`|EnumEquality` _returnvalue "ATTACK"))
    (`self.PlayAnimMontage` (`|GetArrayItem` (`self.RedQueenComboMontage`) (`self.CurComboCount`)) 2.0)
    (`self.BlueprintChangeState` "ATTACK")
    (`/Engine/EditorBlueprintResources/StandardMacros.IncrementInt` (`self.CurComboCount`)
      (:`  `
        (if (== (`self.CurComboCount`) (`KismetArrayLibrary.Array_Length` (`self.RedQueenComboMontage`)))
          (set `self.CurComboCount` 0))))))

(event `self.JumpAttackCombo`
  (bind _returnvalue (`self.BlueprintGetCurState`))
  (if (not (`|EnumEquality` _returnvalue "ATTACK"))
    (`self.PlayAnimMontage` (`|GetArrayItem` (`self.JumpAttackMontage`) (`self.CurComboCount`)) 2.0)
    (`self.BlueprintChangeState` "ATTACK")
    (`/Engine/EditorBlueprintResources/StandardMacros.IncrementInt` (`self.CurComboCount`)
      (:`  `
        (if (== (`self.CurComboCount`) (`KismetArrayLibrary.Array_Length` (`self.JumpAttackMontage`)))
          (set `self.CurComboCount` 0))))))

(event `self.Evade`
  (bind _keydir_x (`KismetMathLibrary.BreakVector2D` (`self.KeyDir`)))
  (bind (_keydir_x_2 _keydir_y) (`KismetMathLibrary.BreakVector2D` (`self.KeyDir`)))
  (bind (_keydir_x_3 _keydir_y_2) (`KismetMathLibrary.BreakVector2D` (`self.KeyDir`)))
  (bind _returnvalue (`self.BlueprintGetCurState`))
  (if (`|EnumEquality` _returnvalue "LOCKON")
    (if (!= _keydir_y_2 0.0)
      (`self.BlueprintChangeState` "EVADE")
      (if (> _keydir_y 0.0)
        (`self.PlayAnimMontage` "/Game/Player/Nero/Anim/Evade/BM_EvadeRight.BM_EvadeRight" 2.0)
        (else
          (`self.PlayAnimMontage` "/Game/Player/Nero/Anim/Evade/BM_EvadeLeft.BM_EvadeLeft" 2.0)))
      (elif (< _keydir_x 0.0)
        (`self.BlueprintChangeState` "JUMPBACK")
        (`self.PlayAnimMontage` "/Game/Player/Nero/Anim/Evade/BM_JumpBack.BM_JumpBack" 2.0)
        (else
          (`self.BlueprintChangeState` "JUMP"))))))

(event `self.ArmChangeAttack`
  (bind _returnvalue (`self.BlueprintGetCurState`))
  (if (`|EnumEquality` _returnvalue "Z_ACTION")
    _
    (elif (`NavMovementComponent.IsFalling` (`self.CharacterMovement`))
      (`self.PlayAnimMontage` "/Game/Player/Nero/Anim/Arm/BM_OvertureShootAir.BM_OvertureShootAir")
      (`self.BlueprintChangeState` "Z_ACTION")
      (else
        (`self.PlayAnimMontage` "/Game/Player/Nero/Anim/Arm/BM_OvertureShoot.BM_OvertureShoot")
        (`self.BlueprintChangeState` "Z_ACTION")))))

(event `self.GunShoot`
  (`self.PlayAnimMontage` "/Game/Player/Nero/Anim/Gun/BM_Shoot.BM_Shoot"))

(event `self.DamagedgeneralAnim`
  (if (`NavMovementInterface.IsFalling` (`self.CharacterMovement`))
    (`self.PlayAnimMontage` "/Game/Player/Nero/Anim/Damaged/BM_Away_Fly.BM_Away_Fly" 2.0)
    (else
      (`self.PlayAnimMontage` "/Game/Player/Nero/Anim/Damaged/BM_Common.BM_Common" 2.0))))

(event `self.DamagedImpulseAnim`
  (if (`NavMovementInterface.IsFalling` (`self.CharacterMovement`))
    (`self.PlayAnimMontage` "/Game/Player/Nero/Anim/Damaged/BM_Away_Fly.BM_Away_Fly" 2.0)
    (else
      (`self.PlayAnimMontage` "/Game/Player/Nero/Anim/Damaged/BM_Away_Ground.BM_Away_Ground" 2.0))))

(fn `Check Fsm`
  (bind _returnvalue (cast `EPlayerState` (`KismetMathLibrary.Conv_IntToByte` (`FsmComponent.GetCurrentState` (`self.FsmComp`)))))
  (if (!= (`self.CurFsm`) (`KismetMathLibrary.Conv_IntToByte` (`FsmComponent.GetCurrentState` (`self.FsmComp`))))
    (set `self.CurFsm` _returnvalue)
    (`KismetSystemLibrary.PrintString` (`|GetEnumeratorNameAsString` _returnvalue))))

(fn `EnemyCameraCheck`
  (returns (ReturnValue :type Boolean))
  (`self.LockOnEnemy`
    (:`then`
      (bind (_outhit _returnvalue) (`KismetSystemLibrary.LineTraceSingleForObjects` (`self.K2_GetActorLocation`) (`self.K2_GetActorLocation` (`self.LockOnEnemy`)) (`self.ObstacleType`)))
      (return _returnvalue))
    (:`else`)))

(fn `EnemyCheck`
  (bind _returnvalue (`self.K2_GetActorLocation`))
  (bind (_outactors _returnvalue_2) (`KismetSystemLibrary.SphereOverlapActors` _returnvalue (`self.SearchRadius`) (`self.PawnType`) "/Script/DevilMayCry.EnemyBase"))
  (if _returnvalue_2
    (bind _asenemy_base (cast `EnemyBase` (`.ReturnValue` (`GameplayStatics.FindNearestActor` _returnvalue _outactors))))
    (bind _returnvalue_3 (`EnemyBase.GetIsDestroy` _asenemy_base))
    (if _returnvalue_3
      (set `self.LockOnEnemy` null)
      (else
        (set `self.LockOnEnemy` _asenemy_base)
        (`self.EnemyCameraCheck`)))
    (else
      (set `self.LockOnEnemy` null))))

(fn `UserConstructionScript`)